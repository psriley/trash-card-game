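; BP_Interactable is a Blueprint in a card game that responds to mouse hover and clicks on its owner, apparently as debug scaffolding.
; On BeginPlay it caches the player pawn's CardPlayerPlayerState, printing an error if the cast fails, then binds the owner's cursor-over and click events.
; Hovering prints the actor's name, while clicking prints the player state's TestBool value.
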(event Custom|OnBeginCursorOver_Event
  (params (TouchedActor :type Actor%20Object%20Reference))
  (Development|PrintString (Utilities|String|Append (Utilities|GetDisplayName TouchedActor) " has been hovered over yo!")))

(event Custom|OnClicked_Event
  (params (TouchedActor :type Actor%20Object%20Reference) (ButtonPressed :type Key%20Structure :default "None"))
  (Development|PrintString (Utilities|String|Append "Test Bool Value: " (Utilities|String|ToString(Boolean) (Variables|/Script/TrashCardGame.CardPlayerPlayerState|GetTestBool (Variables|Default|GetPlayerStateObject))))))

(event EventBeginPlay
  (bind _ascard_player_player_state (Utilities|Casting|CastToCardPlayerPlayerState (Variables|/Script/Engine.Pawn|GetPlayerState (Game|Player|GetPlayerPawn 0)))
    (:then
      (Variables|Default|SetPlayerStateObject _ascard_player_player_state)
      (bind _output_get (Variables|Default|SetCardActor (Components|GetOwner)))
      (EventDispatchers|AssignOnBeginCursorOver _output_get (delegate Custom|OnBeginCursorOver_Event))
      (EventDispatchers|AssignOnClicked _output_get (delegate Custom|OnClicked_Event)))
    (:CastFailed
      (Development|PrintString "ERROR CASTING TO CARDPLAYERPLAYERSTATE!"))))

(event EventTick
  (params (DeltaSeconds :type Float%20%28single-precision%29)))