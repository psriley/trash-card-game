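; Behavior tree task that gathers the actionable cards in an AI card player's layout.
; It stores the player's Layout in the blackboard, then adds each face-down card and each face-up non-wild card to the Layout's ActionableCards map, keyed by index.
; It then finishes successfully.
; A disconnected loop for storing a face-down card in the blackboard never runs.
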(event Custom|FoundFaceDownCard
  (bind _array_element (Utilities|Array|ForEachLoopwithBreak 0) ; enters at Break
    (:LoopBody
      (if (not (Variables|/Script/TrashCardGame.BaseCard|GetfaceUp _array_element))
        (Class|BTFunctionLibrary|SetBlackboardValueasObject (Variables|Default|GetBBKO_FaceDown) _array_element)
        (CallFunction|FoundFaceDownCard)))))

(event EventReceiveExecuteAI
  (params (OwnerController :type AI%20Controller%20Object%20Reference) (ControlledPawn :type Pawn%20Object%20Reference))
  (bind _asaicard_player_controller (Utilities|Casting|CastToAICardPlayerController OwnerController))
  (bind _output_get (Variables|Default|SetLayout (Variables|/Script/TrashCardGame.AICardPlayer|GetLayout (Variables|/Script/TrashCardGame.AICardPlayerController|Getplayer _asaicard_player_controller))))
  (Class|BTFunctionLibrary|SetBlackboardValueasObject (Variables|Default|GetBBKO_CardLayout) _output_get)
  (for (_array_element _array_index) (Variables|/Script/TrashCardGame.CardLayout|Getcards (Variables|Default|GetLayout))
    ;[1 1 1] Add face down and face up wild cards to actionable cards map
    (if (Variables|/Script/TrashCardGame.BaseCard|GetfaceUp _array_element)
      (bind _returnvalue (Class|BaseCard|GetCard _array_element))
      (if (not (Variables|/Script/TrashCardGame.Card|GetIsWild _returnvalue))
        (Utilities|Map|Add (Variables|/Script/TrashCardGame.CardLayout|GetActionableCards (Variables|Default|GetLayout)) _array_index _array_element :!label _label))
      (else
        (goto _label))))
  (AI|BehaviorTree|FinishExecute true))