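; Behavior tree task that places the AI card player's in-hand card into its card layout.
; Wild cards go to a random actionable slot; others go to their rank's slot if it is face down or holds a face-up wild.
; SwapCardInHand sets the slot's card but reassigns the same hand card, ignoring the displaced one, then updates the blackboard.
; The task finishes with whether a card was placed.
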(event EventReceiveExecuteAI
  (params (OwnerController :type AI%20Controller%20Object%20Reference) (ControlledPawn :type Pawn%20Object%20Reference))
  (bind _asaicard_player_controller (Utilities|Casting|CastToAICardPlayerController OwnerController))
  (Variables|Default|SetAIPlayer (Variables|/Script/TrashCardGame.AICardPlayerController|Getplayer _asaicard_player_controller))
  (Variables|Default|SetPlacedCard false)
  (bind _ascard (Utilities|Casting|CastToCard (Class|BTFunctionLibrary|GetBlackboardValueasObject (Variables|Default|GetBBKI_CardInHand))))
  (bind _output_get (Variables|Default|SetLocalCardInHand _ascard))
  (bind _output_get_2 (Variables|Default|SetNewVar (Class|BTFunctionLibrary|GetBlackboardValueasObject (Variables|Default|GetBBKI_CardLayout))))
  (bind _ascard_layout (Utilities|Casting|CastToCardLayout _output_get_2)
    (:then
      (if (Variables|/Script/TrashCardGame.Card|GetIsWild _output_get)
        (if (Utilities|Map|IsEmpty (Variables|/Script/TrashCardGame.CardLayout|GetActionableCards _ascard_layout))
          _
          (else
            (bind _values (Utilities|Map|Values (Variables|/Script/TrashCardGame.CardLayout|GetActionableCards _ascard_layout)))
            (bind _returnvalue (Class|BaseCard|GetCard (.OutItem (Utilities|Array|Random _values))))
            (CallFunction|SwapCardinHand (.OutItem (Utilities|Array|Random _values)) _returnvalue (Variables|Default|GetLocalCardInHand))))
        (elif (<= (- (Variables|/Script/TrashCardGame.Card|GetRank (Variables|Default|GetLocalCardInHand)) 1) 9)
          (Utilities|IsValid (Utilities|Array|Get(acopy) (Variables|/Script/TrashCardGame.CardLayout|Getcards _ascard_layout) (- (Variables|/Script/TrashCardGame.Card|GetRank (Variables|Default|GetLocalCardInHand)) 1))
            (:Is%20Valid
              (bind _returnvalue_2 (Class|BaseCard|GetCard (Utilities|Array|Get(acopy) (Variables|/Script/TrashCardGame.CardLayout|Getcards _ascard_layout) (- (Variables|/Script/TrashCardGame.Card|GetRank (Variables|Default|GetLocalCardInHand)) 1))))
              (if (Variables|/Script/TrashCardGame.BaseCard|GetfaceUp (Utilities|Array|Get(acopy) (Variables|/Script/TrashCardGame.CardLayout|Getcards _ascard_layout) (- (Variables|/Script/TrashCardGame.Card|GetRank (Variables|Default|GetLocalCardInHand)) 1)))
                (if (Variables|/Script/TrashCardGame.Card|GetIsWild _returnvalue_2)
                  (CallFunction|SwapCardinHand (Utilities|Array|Get(acopy) (Variables|/Script/TrashCardGame.CardLayout|Getcards _ascard_layout) (- (Variables|/Script/TrashCardGame.Card|GetRank (Variables|Default|GetLocalCardInHand)) 1)) _returnvalue_2 (Variables|Default|GetLocalCardInHand) :!label _label))
                (else
                  (goto _label))))
            (:Is%20Not%20Valid
              _))))
      (AI|BehaviorTree|FinishExecute (Variables|Default|GetPlacedCard)))
    (:CastFailed
      (Development|PrintString "Failed to cast card layout"))))

(fn SwapCardinHand
  (params (LayoutCardActor :type Base%20Card%20Object%20Reference) (LayoutCardObject :type Card%20Object%20Reference) (OldCardInHand :type Card%20Object%20Reference))
  (bind _aiplayer (Variables|Default|GetAIPlayer))
  (Utilities|IsValid _aiplayer
    (:Is%20Valid
      (bind _output_get (LocalVariables|SetTemp (Variables|/Script/TrashCardGame.AICardPlayer|GetCardInHand _aiplayer)))
      (Class|BaseCard|SetCard LayoutCardActor (Variables|/Script/TrashCardGame.AICardPlayer|GetCardInHand _aiplayer) false)
      (bind _output_get_2 (Variables|/Script/TrashCardGame.AICardPlayer|SetCardInHand (Variables|Default|GetAIPlayer) _output_get))
      (Development|PrintString (Utilities|String|Append "Wild: " (Utilities|String|ToString(Boolean) (Variables|/Script/TrashCardGame.Card|GetIsWild _output_get_2))))
      (Class|BTFunctionLibrary|SetBlackboardValueasObject (Variables|Default|GetBBKI_CardInHand) _output_get_2)
      (Variables|Default|SetPlacedCard true))
    (:Is%20Not%20Valid
      (Development|PrintString "Player doesn't exist when swapping card in hand"))))