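; BP_CardGameMode is the game mode Blueprint for a card game, currently acting as a test of deck creation.
; On BeginPlay it constructs a new card deck object, then prints the card count and the display name of the card at a hardcoded index.
; Tick is disabled and the construction script only calls its parent, so no game rules are implemented here.
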(event EventBeginPlay
  (|CallParentFunction)
  (bind _returnvalue (Game|ConstructObjectfromClass "/Script/TrashCardGame.CardDeck"))
  (Development|PrintString (Utilities|String|ToString(Integer) (Utilities|Array|Length (Variables|/Script/TrashCardGame.CardDeck|Getcards _returnvalue))))
  (bind _output_get (Variables|Default|SetCardsIndex 45))
  (Development|PrintString (Utilities|GetDisplayName (Utilities|Array|Get(acopy) (Variables|/Script/TrashCardGame.CardDeck|Getcards _returnvalue) _output_get))))

(event EventTick
  (params (DeltaSeconds :type Float%20%28single-precision%29))
  (|CallParentFunction DeltaSeconds) ; This node is disabled and will not be called.\nDrag off pins to build functionality.
)

(fn ConstructionScript
  (|CallParentFunction))